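; Leader unit that reports its health to the local player's HUD leader health widget, showing a dark mesh for Team Krampus.
; One second after BeginPlay, it caches the HUD and player state, then seeds max health as own or enemy by team.
; Tick polls the widget updates: game state label, phase timer, this leader's health, and player points when on the same team.
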(event EventBeginPlay
  (if (Utilities|Enum|Equal(Enum) (Variables|Default|GetTeam) "T_Krampus")
    (Rendering|SetVisibility (Variables|Character|GetMesh) false true)
    (Rendering|SetVisibility (Variables|Default|GetMesh_Dark) true true))
  (Utilities|Time|SetTimerbyFunctionName self "DelayedStart" 1.0))

(event Collision|EventActorBeginOverlap
  (params (OtherActor :type Actor%20Object%20Reference)))

(event EventTick
  (params (DeltaSeconds :type Float%20%28single-precision%29))
  (bind _currentplayerstate (Variables|Default|GetCurrentPlayerState))
  (bind _hud (Variables|Default|GetHUD))
  (bind _health (Variables|Default|GetHealth))
  (bind _leaderhealthwidget (Variables|/Game/HUD/BPGameHUD.BPGameHUD_C|GetLeaderHealthWidget _hud))
  (if (Utilities|IsValid _currentplayerstate)
    (bind _asmy_game_state_base (Utilities|Casting|CastToMyGameStateBase (Game|GetGameState))
      (:then
        (Utilities|FlowControl|Sequence
          (:then_0
            (bind _returnvalue (Class|MyGameStateBase|GetStateLabel _asmy_game_state_base))
            (Variables|/Game/HUD/Widgets/LeaderHealth.LeaderHealth_C|SetGameState _leaderhealthwidget (Utilities|Text|ToText(String) _returnvalue)))
          (:then_1
            (bind _returnvalue_2 (Class|MyGameStateBase|GetPhaseTimer _asmy_game_state_base))
            (Variables|/Game/HUD/Widgets/LeaderHealth.LeaderHealth_C|SetPhaseTimer _leaderhealthwidget (Math|Float|Truncate _returnvalue_2)))
          (:then_2
            (if (Utilities|Enum|Equal(Enum) (Class|MyPlayerState|GetTeam _currentplayerstate) (Variables|Default|GetTeam)) :!label _label
              (Variables|/Game/HUD/Widgets/LeaderHealth.LeaderHealth_C|SetMyLeaderHealth _leaderhealthwidget _health)
              (Variables|/Game/HUD/Widgets/LeaderHealth.LeaderHealth_C|SetScore _leaderhealthwidget (Class|MyPlayerState|GetPoints (Variables|Default|GetCurrentPlayerState)))
              (else
                (Variables|/Game/HUD/Widgets/LeaderHealth.LeaderHealth_C|SetEnemyLeaderHealth _leaderhealthwidget _health))))))
      (:CastFailed
        (goto _label)))))

(fn ConstructionScript)

(fn DelayedStart
  (bind _returnvalue (Game|GetPlayerController 0))
  (bind _health (Variables|Default|GetHealth))
  (Variables|Default|SetUnitMesh (Variables|Character|GetMesh))
  (bind _asbpgame_hud (Utilities|Casting|CastToBPGameHUD (HUD|GetHUD _returnvalue)))
  (Variables|Default|SetHUD _asbpgame_hud)
  (bind _asmy_player_state (Utilities|Casting|CastToMyPlayerState (Variables|/Script/Engine.Controller|GetPlayerState _returnvalue))
    (:then
      (bind _output_get (Variables|Default|SetCurrentPlayerState _asmy_player_state))
      (Variables|/Game/HUD/Widgets/LeaderHealth.LeaderHealth_C|SetPlayerState (Variables|/Game/HUD/BPGameHUD.BPGameHUD_C|GetLeaderHealthWidget (Variables|Default|GetHUD)) _output_get)
      (if (Utilities|Enum|Equal(Enum) (Class|MyPlayerState|GetTeam _output_get) (Variables|Default|GetTeam))
        (bind _output_get_2 (Variables|/Game/HUD/Widgets/LeaderHealth.LeaderHealth_C|SetMyLeaderMaxHealth (Variables|/Game/HUD/BPGameHUD.BPGameHUD_C|GetLeaderHealthWidget (Variables|Default|GetHUD)) _health))
        (Variables|/Game/HUD/Widgets/LeaderHealth.LeaderHealth_C|SetMyLeaderHealth (Variables|/Game/HUD/BPGameHUD.BPGameHUD_C|GetLeaderHealthWidget (Variables|Default|GetHUD)) _output_get_2)
        (else
          (bind _output_get_3 (Variables|/Game/HUD/Widgets/LeaderHealth.LeaderHealth_C|SetEnemyLeaderMaxHealth (Variables|/Game/HUD/BPGameHUD.BPGameHUD_C|GetLeaderHealthWidget (Variables|Default|GetHUD)) _health))
          (Variables|/Game/HUD/Widgets/LeaderHealth.LeaderHealth_C|SetEnemyLeaderHealth (Variables|/Game/HUD/BPGameHUD.BPGameHUD_C|GetLeaderHealthWidget (Variables|Default|GetHUD)) _output_get_3))))
    (:CastFailed
      (Development|PrintString "Failed To Cast" true true "(R=0.000000,G=0.660000,B=1.000000,A=1.000000)" 6e+01))))