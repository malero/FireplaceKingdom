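; Brute unit Blueprint that sets up its spawn sound and team-specific appearance.
; On BeginPlay it plays a random entry from its Sounds array and starts a short one-shot timer for CheckMesh.
; CheckMesh hides the default mesh and shows the dark variant when the unit's team is Krampus.
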(event EventBeginPlay
  (bind _audio (Variables|Default|GetAudio))
  (bind _sounds (Variables|Default|GetSounds))
  (Audio|Components|Audio|SetSound _audio (Utilities|Array|Get(acopy) _sounds (Math|Random|RandomIntegerinRange 0 (Utilities|Array|Length _sounds))))
  (Audio|Components|Audio|Play _audio 0.0)
  (Utilities|Time|SetTimerbyFunctionName self "CheckMesh" 0.1))

(event Collision|EventActorBeginOverlap
  (params (OtherActor :type Actor%20Object%20Reference)))

(event EventTick
  (params (DeltaSeconds :type Float%20%28single-precision%29)))

(fn ConstructionScript)

(fn CheckMesh
  (if (Utilities|Enum|Equal(Enum) (Variables|Default|GetTeam) "T_Krampus")
    (Rendering|SetVisibility (Variables|Character|GetMesh) false false)
    (Rendering|SetVisibility (Variables|Default|GetMesh_Dark) true false)))